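; Prototype player controller for a tower game, handling click-drag of towers, party slot allocation and wave starts via Enhanced Input.
; Tick moves the clicked actor under the cursor, projecting the trace hit along the camera ray to the actor's height, and release sends a drop message.
; Slot allocation uses gameplay tags to validate the actor, fills the first of six free slots and updates the party UI widget.
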(event `self.ReceiveTick`
  (params (DeltaSeconds :type "Float (single-precision)"))
  (`self.Isometric Click/Drag Tower Movement`))

(event `EnhancedInput|/Game/RunDekunda/Prototype/BluePrints/input_action/IA_StartWave`
  (params (ActionValue :type Boolean) (ElapsedSeconds :type "Float (double-precision)") (TriggeredSeconds :type "Float (double-precision)") (InputAction :type "InputAction Object Reference" :default "/Game/RunDekunda/Prototype/BluePrints/input_action/IA_StartWave.IA_StartWave"))
  (:`Triggered`
    (bind _enemywave__spawner_ref (`self.EnemyWave  Spawner Ref`)
      (:`then`
        (message `/Game/RunDekunda/Prototype/BluePrints/SpawnWave_BPI.Spawn Wave` _enemywave__spawner_ref))
      (:`else`))))

(event `Reset Refrence Tags`
  ;[0.03692 1 0.179] Tower Slot Allocation
  (set `self.Clicked Actor Gameplay TagsREF` (struct)))

(event `self.ReceiveBeginPlay`
  (`self.Setup Input`))

(event `/Game/RunDekunda/Prototype/BluePrints/Tag_BPI.TriggerTowerSlotAllocation`
  ;[0.03692 1 0.179] Tower Slot Allocation
  (bind _gameplay_tags (message `/Game/RunDekunda/Prototype/BluePrints/Tag_BPI.Get Tags` (`self.Clicked Actor`)))
  (set `self.Clicked Actor Gameplay TagsREF` _gameplay_tags)
  (if (`BlueprintGameplayTagLibrary.HasTag` (`self.Clicked Actor Gameplay TagsREF`) (struct :`TagName` "TowerPartyManagement.CanBePartyMember?"))
    (if (`BlueprintGameplayTagLibrary.HasTag` (`self.Clicked Actor Gameplay TagsREF`) (struct :`TagName` "TowerPartyManagement.CanBePartyMember?.AlreadyInSlot"))
      (`KismetSystemLibrary.PrintString` "Already in slot" true true (struct :`R` 1.0 :`G` 0.040508 :`B` 0.020612 :`A` 1.0))
      (`self.Reset Refrence Tags`)
      (else
        (bind _slotname (`self.Check Tower Slot Avalability` (`self.Clicked Actor`))) ; Runs a check on all slots to see if one is avalable \n- then if one is, set the actor to that slot
        (`KismetSystemLibrary.PrintString` (`KismetStringLibrary.Conv_NameToString` _slotname) true true (struct :`R` 0.036923 :`G` 1.0 :`B` 0.179031 :`A` 1.0))
        (`self.Reset Refrence Tags`)))
    (else
      (`KismetSystemLibrary.PrintString` "Not Compatable" true true (struct :`R` 1.0 :`G` 0.040508 :`B` 0.020612 :`A` 1.0))
      (`self.Reset Refrence Tags`))))

(event `EnhancedInput|/Game/RunDekunda/Prototype/BluePrints/input_action/IA_Click`
  (params (ActionValue :type Boolean) (ElapsedSeconds :type "Float (double-precision)") (TriggeredSeconds :type "Float (double-precision)") (InputAction :type "InputAction Object Reference" :default "/Game/RunDekunda/Prototype/BluePrints/input_action/IA_Click.IA_Click"))
  (bind (_bblockinghit _clickedactor) (`self.GetClickedItem`))
  ;[1 0.8385 0.1289] Input Action Click
  (:`Started`
    (if _bblockinghit
      (`/Engine/EditorBlueprintResources/StandardMacros.IsValid` _clickedactor
        (:`Is Valid`
          (if (`GameplayStatics.BreakHitResult` (`self.GetHitResultUnderCursorByChannel` "TraceTypeQuery1"))
            (set `self.Clicked Actor` _clickedactor))))))
  (:`Completed`
    (message `/Game/RunDekunda/Prototype/BluePrints/Tag_BPI.TriggerTowerDrop` (`self.Clicked Actor`))
    (set `self.Clicked Actor` null)))

(event `EnhancedInput|/Game/RunDekunda/Prototype/BluePrints/input_action/IA_RightClick`
  (params (ActionValue :type Boolean) (ElapsedSeconds :type "Float (double-precision)") (TriggeredSeconds :type "Float (double-precision)") (InputAction :type "InputAction Object Reference" :default "/Game/RunDekunda/Prototype/BluePrints/input_action/IA_RightClick.IA_RightClick"))
  ;[1 0.8385 0.1289] Input Action Click
)

(fn `Check Tower Slot Avalability`
  (params (`Clicked Actor` :type "Actor Object Reference"))
  (returns (SlotName :type Name))
  ;[1 1 1] Run a validated check on every tower slot - if the slot is empty asign the actor to that slot
  (`self.PartyTowerSlot_1`
    (:`then`
      (`self.PartyTowerSlot_2`
        (:`then`
          (`self.PartyTowerSlot_3`
            (:`then`
              (`self.PartyTowerSlot_4`
                (:`then`
                  (`self.PartyTowerSlot_5`
                    (:`then`
                      (`self.PartyTowerSlot_6`
                        (:`then`
                          (return "ALL SLOTS FULL"))
                        (:`else`
                          (set `self.PartyTowerSlot_6` `Clicked Actor`)
                          (`BlueprintGameplayTagLibrary.AddGameplayTag` (`self.Clicked Actor Gameplay TagsREF`) (struct :`TagName` "TowerPartyManagement.CanBePartyMember?.AlreadyInSlot.Slot6"))
                          (message `/Game/RunDekunda/Prototype/BluePrints/Tag_BPI.Update tags` (`self.Clicked Actor`) (`self.Clicked Actor Gameplay TagsREF`))
                          (bind _tower_ui_2d_texture (message `/Game/RunDekunda/Prototype/BluePrints/Tag_BPI.Get UI Icon` (`self.Clicked Actor`)))
                          (`/Game/RunDekunda/Prototype/UI/UI_PartySlots_Prototype.Update Icon` (`self.Slot UI Widget Ref`) 6 _tower_ui_2d_texture)
                          (return "Set Slot 6"))))
                    (:`else`
                      (set `self.PartyTowerSlot_5` `Clicked Actor`)
                      (`BlueprintGameplayTagLibrary.AddGameplayTag` (`self.Clicked Actor Gameplay TagsREF`) (struct :`TagName` "TowerPartyManagement.CanBePartyMember?.AlreadyInSlot.Slot5"))
                      (message `/Game/RunDekunda/Prototype/BluePrints/Tag_BPI.Update tags` (`self.Clicked Actor`) (`self.Clicked Actor Gameplay TagsREF`))
                      (bind _tower_ui_2d_texture_2 (message `/Game/RunDekunda/Prototype/BluePrints/Tag_BPI.Get UI Icon` (`self.Clicked Actor`)))
                      (`/Game/RunDekunda/Prototype/UI/UI_PartySlots_Prototype.Update Icon` (`self.Slot UI Widget Ref`) 5 _tower_ui_2d_texture_2)
                      (return "Set Slot 5"))))
                (:`else`
                  (set `self.PartyTowerSlot_4` `Clicked Actor`)
                  (`BlueprintGameplayTagLibrary.AddGameplayTag` (`self.Clicked Actor Gameplay TagsREF`) (struct :`TagName` "TowerPartyManagement.CanBePartyMember?.AlreadyInSlot.Slot4"))
                  (message `/Game/RunDekunda/Prototype/BluePrints/Tag_BPI.Update tags` (`self.Clicked Actor`) (`self.Clicked Actor Gameplay TagsREF`))
                  (bind _tower_ui_2d_texture_3 (message `/Game/RunDekunda/Prototype/BluePrints/Tag_BPI.Get UI Icon` (`self.Clicked Actor`)))
                  (`/Game/RunDekunda/Prototype/UI/UI_PartySlots_Prototype.Update Icon` (`self.Slot UI Widget Ref`) 4 _tower_ui_2d_texture_3)
                  (return "Set Slot 4"))))
            (:`else`
              (set `self.PartyTowerSlot_3` `Clicked Actor`)
              (`BlueprintGameplayTagLibrary.AddGameplayTag` (`self.Clicked Actor Gameplay TagsREF`) (struct :`TagName` "TowerPartyManagement.CanBePartyMember?.AlreadyInSlot.Slot3"))
              (message `/Game/RunDekunda/Prototype/BluePrints/Tag_BPI.Update tags` (`self.Clicked Actor`) (`self.Clicked Actor Gameplay TagsREF`))
              (bind _tower_ui_2d_texture_4 (message `/Game/RunDekunda/Prototype/BluePrints/Tag_BPI.Get UI Icon` (`self.Clicked Actor`)))
              (`/Game/RunDekunda/Prototype/UI/UI_PartySlots_Prototype.Update Icon` (`self.Slot UI Widget Ref`) 3 _tower_ui_2d_texture_4)
              (return "Set Slot 3"))))
        (:`else`
          (set `self.PartyTowerSlot_2` `Clicked Actor`)
          (`BlueprintGameplayTagLibrary.AddGameplayTag` (`self.Clicked Actor Gameplay TagsREF`) (struct :`TagName` "TowerPartyManagement.CanBePartyMember?.AlreadyInSlot.Slot2"))
          (message `/Game/RunDekunda/Prototype/BluePrints/Tag_BPI.Update tags` (`self.Clicked Actor`) (`self.Clicked Actor Gameplay TagsREF`))
          (bind _tower_ui_2d_texture_5 (message `/Game/RunDekunda/Prototype/BluePrints/Tag_BPI.Get UI Icon` (`self.Clicked Actor`)))
          (`/Game/RunDekunda/Prototype/UI/UI_PartySlots_Prototype.Update Icon` (`self.Slot UI Widget Ref`) 2 _tower_ui_2d_texture_5)
          (return "Set Slot 2"))))
    (:`else`
      (set `self.PartyTowerSlot_1` `Clicked Actor`)
      (`BlueprintGameplayTagLibrary.AddGameplayTag` (`self.Clicked Actor Gameplay TagsREF`) (struct :`TagName` "TowerPartyManagement.CanBePartyMember?.AlreadyInSlot.Slot1"))
      (message `/Game/RunDekunda/Prototype/BluePrints/Tag_BPI.Update tags` (`self.Clicked Actor`) (`self.Clicked Actor Gameplay TagsREF`))
      (bind _tower_ui_2d_texture_6 (message `/Game/RunDekunda/Prototype/BluePrints/Tag_BPI.Get UI Icon` (`self.Clicked Actor`)))
      (`/Game/RunDekunda/Prototype/UI/UI_PartySlots_Prototype.Update Icon` (`self.Slot UI Widget Ref`) 1 _tower_ui_2d_texture_6)
      (return "Set Slot 1"))))

(fn `Get Tags`
  (returns (`Gameplay Tags` :type "GameplayTagContainer Structure"))
  (return))

(fn `Get UI Icon`
  (returns (`Tower UI 2d texture` :type "Texture2D Object Reference"))
  (return null))

(fn `GetClickedItem`
  (returns (bBlockingHit :type Boolean) (ClickedActor :type "Actor Object Reference"))
  (bind (_bblockinghit _binitialoverlap _time _distance _location _impactpoint _normal _impactnormal _physmat _hitactor) (`GameplayStatics.BreakHitResult` (`self.GetHitResultUnderCursorByChannel` "TraceTypeQuery3")))
  (return _bblockinghit _hitactor))

(fn `Isometric Click/Drag Tower Movement`
  (bind (_returnvalue_x _returnvalue_y _returnvalue_z) (`KismetMathLibrary.BreakVector` (`self.K2_GetActorLocation` (`self.Clicked Actor`))))
  (bind _returnvalue (`self.K2_GetActorLocation` (`GameplayStatics.GetPlayerCameraManager` 0)))
  (bind _returnvalue_2 (- (`self.K2_GetActorLocation` (`GameplayStatics.GetPlayerCameraManager` 0)) (`self.DeprojectMousePositionToWorld` (`GameplayStatics.GetPlayerController` 0))))
  (`/Engine/EditorBlueprintResources/StandardMacros.IsValid` (`self.Clicked Actor`)
    (:`Is Valid`
      (bind (_outhit _returnvalue_3) (`KismetSystemLibrary.LineTraceSingle` _returnvalue (+ _returnvalue (* (- (`self.DeprojectMousePositionToWorld` (`GameplayStatics.GetPlayerController` 0)) _returnvalue) 5000.0)) "TraceTypeQuery1"))
      (if _returnvalue_3
        (bind (_bblockinghit _binitialoverlap _time _distance _location) (`GameplayStatics.BreakHitResult` _outhit))
        (bind _x (.x (+ _location (* _returnvalue_2 (/ (- _returnvalue_z (.z _location)) (.z _returnvalue_2))))))
        (bind _y (.y (+ _location (* _returnvalue_2 (/ (- _returnvalue_z (.z _location)) (.z _returnvalue_2))))))
        (bind _z (.z (+ _location (* _returnvalue_2 (/ (- _returnvalue_z (.z _location)) (.z _returnvalue_2))))))
        (`KismetSystemLibrary.DrawDebugSphere` (`KismetMathLibrary.MakeVector` _x _y _z))
        (`self.K2_SetActorLocation` (`self.Clicked Actor`) (`KismetMathLibrary.MakeVector` _x _y _z) false false)))))

(fn `Set is overlapping tower`
  (returns (TowerSlotOut :type "Object Object Reference") (SnapTransform :type "Transform Structure"))
  (return null))

(fn `SetSpawner`
  (params (Spawner_IN :type "/Game/RunDekunda/Prototype/Actors/EnemySpawner Object Reference"))
  (returns (Spawner_out :type "/Game/RunDekunda/Prototype/Actors/EnemySpawner Object Reference"))
  (return null))

(fn `Setup Input`
  (bind _returnvalue (subsystem `EnhancedInputLocalPlayerSubsystem`))
  (`/Engine/EditorBlueprintResources/StandardMacros.IsValid` _returnvalue
    (:`Is Valid`
      (`EnhancedInputSubsystemInterface.AddMappingContext` _returnvalue "/Game/RunDekunda/Prototype/BluePrints/input_action/Click_AM.Click_AM" 0 (struct))
      (bind _returnvalue_2 (`GameplayStatics.GetActorOfClass` "/Game/RunDekunda/Prototype/Actors/EnemySpawner.EnemySpawner_C"))
      (set `self.EnemyWave  Spawner Ref` _returnvalue_2)
      (bind _returnvalue_3 (`|CreateWidget` "/Game/RunDekunda/Prototype/UI/UI_PartySlots_Prototype.UI_PartySlots_Prototype_C"))
      (bind _output_get (set `self.Slot UI Widget Ref` _returnvalue_3))
      (`UserWidget.AddToViewport` _output_get 0))))

(fn `Update tags`
  (params (`in tags` :type "GameplayTagContainer Structure"))
  (return))

(fn `UserConstructionScript`)