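; A homing projectile that damages enemy units it overlaps.
; On BeginPlay, a valid Target becomes the movement component's homing target and starts a short self-destruct delay, so projectiles without one get no timeout here.
; Sphere overlaps cast the sweep's hit actor to BP_EnemyUnitBase, spawn an explosion emitter at that actor, destroy the projectile, then apply fixed damage.
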(event `self.ReceiveBeginPlay`
  (bind _target (`self.Target`)
    (:`then`
      (set `ProjectileMovementComponent.HomingTargetComponent` (`Actor.RootComponent` _target) (`self.ProjectileMovement`))
      (`KismetSystemLibrary.Delay` 3.0) ; destroy if havent hti anything in 10 secounds
      (`self.K2_DestroyActor`))
    (:`else`)))

(event `self.Sphere_Collision.OnComponentBeginOverlap`
  (params (OverlappedComponent :type "PrimitiveComponent Object Reference") (OtherActor :type "Actor Object Reference") (OtherComp :type "PrimitiveComponent Object Reference") (OtherBodyIndex :type Integer) (bFromSweep :type Boolean) (SweepResult :type "HitResult Structure (by ref)"))
  (bind (_bblockinghit _binitialoverlap _time _distance _location _impactpoint _normal _impactnormal _physmat _hitactor) (`GameplayStatics.BreakHitResult` SweepResult))
  (bind _asbp_enemy_unit_base (cast `/Game/RunDekunda/Prototype/Actors/Enemy_Towers/BP_EnemyUnitBase` _hitactor))
  (if (== _asbp_enemy_unit_base _hitactor)
    (`GameplayStatics.SpawnEmitterAtLocation` "/Game/StarterContent/Particles/P_Explosion.P_Explosion" (`self.K2_GetActorLocation` _hitactor))
    (`self.K2_DestroyActor`)
    (`GameplayStatics.ApplyDamage` _hitactor 25.0 null self)))

(fn `UserConstructionScript`)