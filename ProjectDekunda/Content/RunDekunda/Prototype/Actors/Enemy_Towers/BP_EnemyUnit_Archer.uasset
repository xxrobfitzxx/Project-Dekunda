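; BP_EnemyUnit_Archer is an archer enemy unit Blueprint in the RunDekunda prototype's Enemy_Towers actors.
; Its event graph holds only disabled default events, and its construction script just calls the parent, so no archer-specific behavior is defined here.
; The EnemyPath function assigns the given path only when the stored Path is invalid, then returns Path, so an existing valid path is never replaced.
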(fn `EnemyPath`
  (params (`NewPath?` :type "/Game/RunDekunda/Prototype/Enviroment/BP_Spline Object Reference"))
  (returns (PathSpline :type "/Game/RunDekunda/Prototype/Enviroment/BP_Spline Object Reference"))
  (bind _path (`self.Path`))
  (`/Engine/EditorBlueprintResources/StandardMacros.IsValid` _path
    (:`Is Valid`
      (bind _output_get (set `self.Path` _path))
      (return _output_get))
    (:`Is Not Valid`
      (bind _output_get_2 (set `self.Path` `NewPath?`))
      (return _output_get_2))))

(fn `UserConstructionScript`
  (`parent.UserConstructionScript`))