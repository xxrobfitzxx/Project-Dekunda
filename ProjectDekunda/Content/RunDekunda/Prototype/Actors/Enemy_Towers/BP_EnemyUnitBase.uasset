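; Base Blueprint for enemy units in the RunDekunda prototype, handling health, death, capture and spawner bookkeeping.
; Any damage lowers health and refreshes the HP bar, and zero health triggers death with an explosion.
; Death and capture share a tail that tells the assigned spawner to decrease its alive count, then destroys the actor.
; Setters assign the spawner and a path, keeping any path already valid.
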(event `self.ReceiveActorBeginOverlap`
  (params (OtherActor :type "Actor Object Reference"))
  (`parent.ReceiveActorBeginOverlap` OtherActor))

(event `self.ReceiveAnyDamage`
  (params (Damage :type "Float (single-precision)") (DamageType :type "DamageType Object Reference") (InstigatedBy :type "Controller Object Reference") (DamageCauser :type "Actor Object Reference"))
  ;[1 0.04051 0.02061] Damage
  (if (> (`self.Unit Health`) 0.0)
    (set `self.Unit Health` (- (`self.Unit Health`) Damage))
    (`self.Update Hp_Bar UI`))
  (if (<= (`self.Unit Health`) 0.0)
    (`self.Death`)))

(event `/Game/RunDekunda/Prototype/BluePrints/BPI/TowerManagement_BPI.Captured Enemy`
  ;[1 0.8385 0.1289] Death / captured
  (message `/Game/RunDekunda/Prototype/BluePrints/BPI/SpawnWave_BPI.Decrease total Enemies alive` (`self.Spawner Ref`) :!label _label) ; needs ref
  (`self.K2_DestroyActor`))

(event `Death`
  ;[1 0.8385 0.1289] Death / captured
  (`GameplayStatics.SpawnEmitterAtLocation` "/Game/StarterContent/Particles/P_Explosion.P_Explosion" (`SceneComponent.K2_GetComponentLocation` (`self.Cube`)) (struct) (3.0 3.0 3.0))
  (goto _label))

(fn `EnemyPath`
  (params (`NewPath?` :type "/Game/RunDekunda/Prototype/Enviroment/BP_Spline Object Reference"))
  (returns (PathSpline :type "/Game/RunDekunda/Prototype/Enviroment/BP_Spline Object Reference"))
  (bind _path (`self.Path`))
  (`/Engine/EditorBlueprintResources/StandardMacros.IsValid` _path
    (:`Is Valid`
      (bind _output_get (set `self.Path` _path))
      (return _output_get))
    (:`Is Not Valid`
      (bind _output_get_2 (set `self.Path` `NewPath?`))
      (return _output_get_2))))

(fn `SetSpawner`
  (params (Spawner_IN :type "/Game/RunDekunda/Prototype/Actors/EnemySpawner Object Reference"))
  (returns (Spawner_out :type "/Game/RunDekunda/Prototype/Actors/EnemySpawner Object Reference"))
  (bind _output_get (set `self.Spawner Ref` Spawner_IN))
  (return _output_get))

(fn `UserConstructionScript`
  (`parent.UserConstructionScript`))