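; BP_TowerMaker is a prototype tower slot actor that marks a spot where a tower can snap into place.
; Any actor beginning overlap makes it trigger a tower slot allocation message on player controller 0, with no filter on the overlapping actor.
; Set is overlapping tower returns the actor itself as the slot and its Box world transform as the snap transform.
; The tag and UI icon functions are empty stubs.
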(event `self.ReceiveActorBeginOverlap`
  (params (OtherActor :type "Actor Object Reference"))
  (message `/Game/RunDekunda/Prototype/BluePrints/TowerManagement_BPI.TriggerTowerSlotAllocation` (`GameplayStatics.GetPlayerController` 0)))

(fn `Get Tags`
  (returns (`Gameplay Tags` :type "GameplayTagContainer Structure"))
  (return))

(fn `Get UI Icon`
  (returns (`Tower UI 2d texture` :type "Texture2D Object Reference"))
  (return null))

(fn `Set is overlapping tower`
  (returns (TowerSlotOut :type "Object Object Reference") (SnapTransform :type "Transform Structure"))
  (return self (`SceneComponent.K2_GetComponentToWorld` (`self.Box`))))

(fn `Update tags`
  (params (`in tags` :type "GameplayTagContainer Structure"))
  (return))

(fn `UserConstructionScript`)